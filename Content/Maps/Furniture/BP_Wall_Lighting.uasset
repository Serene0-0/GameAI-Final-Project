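; Wall light fixture that can be broken, creating noise that AI hearing can pick up.
; On BeginPlay a hard-coded true branch turns the point light on.
; BreakLight hides the point light and WallLight, spawns sparks, plays an attenuated smash sound and clears IsLit.
; It also reports a tagged "LightBroken" noise event at the fixture, with the player character as instigator.
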(event `self.ReceiveBeginPlay`
  (if true
    (`SceneComponent.SetVisibility` (`self.PointLight`) true false)
    (else
      (`SceneComponent.SetVisibility` (`self.PointLight`) false false))))

(event `BreakLight`
  (`SceneComponent.SetVisibility` (`self.PointLight`) false false)
  (`GameplayStatics.SpawnEmitterAtLocation` "/Game/StarterContent/Particles/P_Sparks.P_Sparks" (`self.K2_GetActorLocation`))
  (`GameplayStatics.PlaySoundAtLocation` "/Game/Maps/Furniture/148075__sandyrb__lightbulb-smash-001.148075__sandyrb__lightbulb-smash-001" (`self.K2_GetActorLocation`) (struct) 1.0 1.2 0.0 "/Game/Maps/Furniture/SA_Wall_Lighting.SA_Wall_Lighting" null null null)
  (`AISense_Hearing.ReportNoiseEvent` (`self.K2_GetActorLocation`) 0.7 (`GameplayStatics.GetPlayerCharacter` 0) 1000.0 "LightBroken")
  (`SceneComponent.SetVisibility` (`self.WallLight`) false false)
  (set `self.IsLit` false))

(fn `UserConstructionScript`)