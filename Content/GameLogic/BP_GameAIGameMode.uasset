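; BP_GameAIGameMode is a game mode that runs a countdown and declares victory when time runs out.
; Tick decrements RemainingTime, clamped at zero, until it expires and sets the GameOver flag, which stops further updates.
; On expiry it adds WBP_Victory to the viewport for the first PlayerController found, switches input to UI only and shows the mouse cursor.
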(event `self.ReceiveTick`
  (params (DeltaSeconds :type "Float (single-precision)"))
  (if (not (`self.bGameOver`))
    (set `self.RemainingTime` (`KismetMathLibrary.FMax` (- (`self.RemainingTime`) DeltaSeconds)))
    (if (<= (`self.RemainingTime`) 0.0)
      (set `self.bGameOver` true)
      (set `self.RemainingTime` 0.0)
      (bind _outactors (`GameplayStatics.GetAllActorsOfClass` "/Script/Engine.PlayerController"))
      (bind _output (`|GetArrayItem` _outactors))
      (bind _returnvalue (`|CreateWidget` "/Game/UI/WBP_Victory.WBP_Victory_C" _output))
      (`UserWidget.AddToViewport` _returnvalue 0)
      (`WidgetBlueprintLibrary.SetInputMode_UIOnlyEx` _output null)
      (set `PlayerController.bShowMouseCursor` true _output))))

(fn `UserConstructionScript`)